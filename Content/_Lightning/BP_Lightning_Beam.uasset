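; Lightning beam actor that fires a one-time burst of about a hundred Niagara lightning strikes on BeginPlay, then destroys its root component.
; Each strike starts at a random downward offset from the actor, scaled by RandomPlane, and traces toward the actor's Y/Z at world X zero.
; The spawned system receives start, end and fixed upward normal parameters, using the trace impact as end or world origin on a miss.
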(event `self.ReceiveBeginPlay`
  (for _ (range 101)
    (`self.Summon_Lightning`))
  (`ActorComponent.K2_DestroyComponent` (`self.DefaultSceneRoot`)))

(fn `Summon_Lightning`
  (locals (RandoDir :type "Vector Structure"))
  (bind _returnvalue (+ (`self.K2_GetActorLocation`) (* (`local.RandoDir`) (`self.RandomPlane`))))
  (set `local.RandoDir` (`KismetMathLibrary.MakeVector` (.x (`KismetMathLibrary.RandomUnitVector`)) (.y (`KismetMathLibrary.RandomUnitVector`)) (* (`KismetMathLibrary.Abs` (.z (`KismetMathLibrary.RandomUnitVector`))) -1.0)))
  (bind _outhit (`KismetSystemLibrary.LineTraceSingle` :`Start` _returnvalue :`End` (`KismetMathLibrary.MakeVector` 0.0 (.y (`self.K2_GetActorLocation`)) (.z (`self.K2_GetActorLocation`))) :`TraceChannel` "TraceTypeQuery1" :`DrawTime` 0.5))
  (bind _returnvalue_2 (`NiagaraFunctionLibrary.SpawnSystemAttached` "/Game/_Lightning/NS_Lightning_Strike.NS_Lightning_Strike" (`self.DefaultSceneRoot`) "None" (0.0 0.0 0.0) (struct) "KeepRelativeOffset"))
  (`NiagaraComponent.SetVariableVec3` _returnvalue_2 "BeamStartPoint" _returnvalue)
  (`NiagaraComponent.SetVariableVec3` _returnvalue_2 "ImpactNormal" (0.0 0.0 1.0))
  (bind (_bblockinghit _binitialoverlap _time _distance _location _impactpoint) (`GameplayStatics.BreakHitResult` _outhit))
  (if _bblockinghit
    (`NiagaraComponent.SetVariableVec3` _returnvalue_2 "BeamEndPoint" _impactpoint)
    (else
      (`NiagaraComponent.SetVariableVec3` _returnvalue_2 "BeamEndPoint" (0.0 0.0 0.0)))))

(fn `UserConstructionScript`)
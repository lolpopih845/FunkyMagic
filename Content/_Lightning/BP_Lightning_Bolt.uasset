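; Lightning bolt actor that fires a short burst of visual lightning strikes along a direction passed in through Init, then destroys itself after a delay.
; Tick runs a cooldown that repeatedly calls SummonLightning until the strike limit is reached.
; Each strike line-traces forward from a jittered origin and spawns a Niagara beam ending at the hit point or max range.
; The computed random downward direction is unused.
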(event `self.ReceiveTick`
  (params (DeltaSeconds :type "Float (single-precision)"))
  (if (> (`self.Strike`) 6)
    (`KismetSystemLibrary.Delay` 2.0)
    (`self.K2_DestroyActor`)
    (else
      (bind _output_get (set `self.Cd` (- (`self.Cd`) DeltaSeconds)))
      (if (< _output_get 0.0)
        (set `self.Cd` 0.3)
        (`self.Summon_Lightning`)
        (set `self.Strike` (+ (`self.Strike`) 1))))))

(event `Init`
  (params (Init :type "Vector Structure"))
  (set `self.FrontPos` Init))

(fn `Summon_Lightning`
  (locals (RandoDir :type "Vector Structure"))
  (bind _returnvalue (+ (`self.K2_GetActorLocation`) (* (`KismetMathLibrary.RandomUnitVector`) (75.0 75.0 75.0))))
  (bind _returnvalue_2 (+ (`self.K2_GetActorLocation`) (* (`self.FrontPos`) (5000.0 5000.0 5000.0))))
  (set `local.RandoDir` (`KismetMathLibrary.MakeVector` (.x (`KismetMathLibrary.RandomUnitVector`)) (.y (`KismetMathLibrary.RandomUnitVector`)) (* (`KismetMathLibrary.Abs` (.z (`KismetMathLibrary.RandomUnitVector`))) -1.0)))
  (bind _outhit (`KismetSystemLibrary.LineTraceSingle` :`Start` _returnvalue :`End` _returnvalue_2 :`TraceChannel` "TraceTypeQuery1" :`DrawTime` 0.5))
  (bind _returnvalue_3 (`NiagaraFunctionLibrary.SpawnSystemAttached` "/Game/_FunkyMagic/_Lightning/NS_Lightning_Strike.NS_Lightning_Strike" (`self.DefaultSceneRoot`) "None" (0.0 0.0 0.0) (struct) "KeepRelativeOffset"))
  (`NiagaraComponent.SetVariableVec3` _returnvalue_3 "BeamStartPoint" _returnvalue)
  (`NiagaraComponent.SetVariableVec3` _returnvalue_3 "ImpactNormal" (0.0 0.0 1.0))
  (bind (_bblockinghit _binitialoverlap _time _distance _location _impactpoint) (`GameplayStatics.BreakHitResult` _outhit))
  (if _bblockinghit
    (`NiagaraComponent.SetVariableVec3` _returnvalue_3 "BeamEndPoint" _impactpoint)
    (else
      (`NiagaraComponent.SetVariableVec3` _returnvalue_3 "BeamEndPoint" _returnvalue_2))))

(fn `UserConstructionScript`)
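; BP_WaterBomb is a thrown water bomb projectile actor that bursts into a splash on impact.
; Init stores an aim vector, waits briefly while any attachment holds, then FireWater detaches it and activates ProjectileMovement with a fixed forward speed and an upward arc adjusted by the aim's Z.
; A hit on the Ball component spawns a Niagara splash at the impact point and destroys the actor, with a delayed self-destroy as fallback.
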(event `WaitToDestroy`
  (`self.K2_DestroyActor`))

(event `FireWater`
  (`self.K2_DetachFromActor` "KeepWorld" "KeepWorld" "KeepWorld")
  (`ProjectileMovementComponent.SetVelocityInLocalSpace` (`self.ProjectileMovement`) (`KismetMathLibrary.MakeVector` 1000.0 0.0 (+ (* (.z (`self.FrontPos`)) 1000.0) 500.0)))
  (`ActorComponent.Activate` (`self.ProjectileMovement`) false))

(event `Init`
  (params (FrontPos :type "Vector Structure"))
  (set `self.FrontPos` FrontPos)
  (`KismetSystemLibrary.Delay` 1.5)
  (`self.FireWater`)
  (`KismetSystemLibrary.Delay` 7.5)
  (`self.WaitToDestroy`))

(event `self.Ball.OnComponentHit`
  (params (HitComponent :type "PrimitiveComponent Object Reference") (OtherActor :type "Actor Object Reference") (OtherComp :type "PrimitiveComponent Object Reference") (NormalImpulse :type "Vector Structure") (Hit :type "HitResult Structure (by ref)"))
  (`NiagaraFunctionLibrary.SpawnSystemAtLocation` "/Game/_FunkyMagic/_Exploding/NS_WaterSplash.NS_WaterSplash" (`.ImpactPoint` (`GameplayStatics.BreakHitResult` Hit)))
  (`self.K2_DestroyActor`))

(fn `UserConstructionScript`)
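; Lightning ball projectile that waits out a short delay, then drifts along the direction passed to Init while crackling with arcs.
; Tick moves it by unswept world offset and runs UpdateTraces on a cooldown.
; Each trace casts a random downward-biased line and, on a hit, spawns an attached Niagara arc with beam endpoints and impact normal.
; A hit on the Yippee component spawns a thunder splash and destroys the actor.
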(event `self.Yippee.OnComponentHit`
  (params (HitComponent :type "PrimitiveComponent Object Reference") (OtherActor :type "Actor Object Reference") (OtherComp :type "PrimitiveComponent Object Reference") (NormalImpulse :type "Vector Structure") (Hit :type "HitResult Structure (by ref)"))
  (`NiagaraFunctionLibrary.SpawnSystemAtLocation` "/Game/_FunkyMagic/_Exploding/NS_ThunderSplash.NS_ThunderSplash" (`.ImpactPoint` (`GameplayStatics.BreakHitResult` Hit)))
  (`self.K2_DestroyActor`))

(event `self.ReceiveTick`
  (params (DeltaSeconds :type "Float (single-precision)"))
  (bind _output_get (set `self.StartRunning` (- (`self.StartRunning`) DeltaSeconds)))
  (`self.UpdateTraces`)
  (if (< _output_get 0.0)
    (`SceneComponent.K2_AddWorldOffset` (`self.DefaultSceneRoot`) (* DeltaSeconds (* (`self.FrontPos`) 150.0)) false false)))

(event `Init`
  (params (FrontPos :type "Vector Structure"))
  (set `self.FrontPos` FrontPos))

(fn `UpdateTraces`
  (locals (RandomDirection :type "Vector Structure" :default (0.0 0.0 0.0)) (ImpactOffset :type "Float (double-precision)" :default 1.0))
  (bind _returnvalue (`self.K2_GetActorLocation`))
  (bind _returnvalue_2 (+ _returnvalue (* (`local.RandomDirection`) (`self.MinRadius`))))
  ; Check Cooldown
  (if (>= (- (`GameplayStatics.GetTimeSeconds`) (`self.LastTrace`)) (`self.TraceCooldown`))
    ; Trace
    (set `local.RandomDirection` (`KismetMathLibrary.MakeVector` (.x (`KismetMathLibrary.RandomUnitVector`)) (.y (`KismetMathLibrary.RandomUnitVector`)) (* (`KismetMathLibrary.Abs` (.z (`KismetMathLibrary.RandomUnitVector`))) -1.0)))
    (bind _outhit (`KismetSystemLibrary.LineTraceSingle` :`Start` _returnvalue_2 :`End` (+ _returnvalue (* (`local.RandomDirection`) (`self.MaxRadius`))) :`TraceChannel` "TraceTypeQuery1" :`DrawTime` (`self.TraceCooldown`)))
    ; Reset Cooldown
    (set `self.LastTrace` (`GameplayStatics.GetTimeSeconds`))
    (bind (_bblockinghit _binitialoverlap _time _distance _location _impactpoint _normal _impactnormal) (`GameplayStatics.BreakHitResult` _outhit))
    ; Spawn NS and Set Parameter
    (if _bblockinghit
      (bind _returnvalue_3 (`NiagaraFunctionLibrary.SpawnSystemAttached` "/Game/_FunkyMagic/_Lightning/NS_LightningArcs.NS_LightningArcs" (`self.DefaultSceneRoot`) "None" (0.0 0.0 0.0) (struct) "KeepRelativeOffset" true))
      (`NiagaraComponent.SetVariableVec3` _returnvalue_3 "BeamStartPoint" _returnvalue_2)
      (`NiagaraComponent.SetVariableVec3` _returnvalue_3 "BeamEndPoint" (+ _impactpoint (* _impactnormal (`local.ImpactOffset`))))
      (`NiagaraComponent.SetVariableVec3` _returnvalue_3 "ImpactNormal" _impactnormal))))

(fn `UserConstructionScript`)
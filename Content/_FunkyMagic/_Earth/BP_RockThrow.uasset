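; BP_RockThrow is an earth magic spawner that releases a short volley of BP_MagicRock actors.
; Init stores a front position, moves the spawner to the given position and starts a Tick-driven countdown.
; At a fixed interval, it adds a child actor component at a random spherical offset and passes the front position to that rock's Init, stopping once the rock count cap is reached.
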(event `self.ReceiveTick`
  (params (DeltaSeconds :type "Float (single-precision)"))
  (if (`self.Start`)
    (if (not (> (`self.rockCount`) 6))
      (bind _output_get (set `self.timey` (- (`self.timey`) DeltaSeconds)))
      (if (< _output_get 0.0)
        (set `self.timey` 0.3)
        (bind _returnvalue (`AddComponent|NODE_AddChildActorComponent-1` :`RelativeTransform` (`KismetMathLibrary.MakeTransform` (* (`KismetMathLibrary.RandomUnitVector`) 100.0))))
        (bind _asbp_magic_rock (cast `/Game/_FunkyMagic/_Earth/BP_MagicRock` (`ChildActorComponent.ChildActor` _returnvalue)))
        (`/Game/_FunkyMagic/_Earth/BP_MagicRock.Init` _asbp_magic_rock (`self.FrontPos`))
        (set `self.rockCount` (+ (`self.rockCount`) 1))))))

(event `Init`
  (params (FrontPos :type "Vector Structure") (Position :type "Vector Structure"))
  (set `self.FrontPos` FrontPos)
  (bind _output_get (set `self.Position` Position))
  (`self.K2_SetActorLocation` _output_get false true)
  (set `self.Start` true))

(fn `UserConstructionScript`
  (locals (FaceVector :type "Vector Structure") (Postion :type "Vector Structure")))
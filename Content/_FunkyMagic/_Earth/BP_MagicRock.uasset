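; BP_MagicRock is an earth-magic rock projectile that is thrown toward a target position.
; Init stores the target, rotates and hides the stone, spawns a Niagara throw effect, then reveals the stone and starts movement after timed delays.
; Tick offsets the stone without sweep by its remaining distance to the target, so it slows on approach.
; A component hit broadcasts OnProjectileImpact, spawns an explosion and destroys the actor.
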(event `self.stone1.OnComponentHit`
  (params (HitComponent :type "PrimitiveComponent Object Reference") (OtherActor :type "Actor Object Reference") (OtherComp :type "PrimitiveComponent Object Reference") (NormalImpulse :type "Vector Structure") (Hit :type "HitResult Structure (by ref)"))
  (`self.OnProjectileImpact` OtherActor Hit)
  (`GameplayStatics.SpawnEmitterAtLocation` "/Game/StarterContent/Particles/P_Explosion.P_Explosion" (`SceneComponent.K2_GetComponentLocation` (`self.stone1`)))
  (`self.K2_DestroyActor`))

(event `Init`
  (params (FrontPos :type "Vector Structure"))
  (set `self.FrontPos` FrontPos)
  (`SceneComponent.K2_SetRelativeRotation` (`self.stone1`) (`KismetMathLibrary.Conv_VectorToRotator` (`KismetMathLibrary.MakeVector` (.y (`self.FrontPos`)) (.x (`self.FrontPos`)) (.z (`self.FrontPos`)))) false false)
  (`SceneComponent.SetVisibility` (`self.stone1`) false false)
  (`NiagaraFunctionLibrary.SpawnSystemAttached` "/Game/_FunkyMagic/_Earth/NS_RockThrow.NS_RockThrow" (`self.DefaultSceneRoot`) "None" (0.0 0.0 -100.0) (struct) "KeepRelativeOffset" true)
  (`KismetSystemLibrary.Delay` 1.0)
  (`SceneComponent.SetVisibility` (`self.stone1`) true false)
  (`KismetSystemLibrary.Delay` 0.5)
  (set `self.StartingMoving` true))

(event `self.ReceiveTick`
  (params (DeltaSeconds :type "Float (single-precision)"))
  (if (`self.StartingMoving`)
    (`SceneComponent.K2_AddWorldOffset` (`self.stone1`) (* DeltaSeconds (* (- (`self.FrontPos`) (`SceneComponent.K2_GetComponentLocation` (`self.stone1`))) 1.0)) false false)))

(fn `UserConstructionScript`)
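; BP_WaterSplash is a magic water projectile that leaves a water pool where it lands.
; Init attaches the NS_water_splash effect to the player near the hand, then after a short delay launches the projectile forward in local space, with vertical speed taken from the aim vector.
; When the sphere collider hits, it spawns and initializes BP_WaterPool at the impact's XY, pinned just above world zero height, then destroys itself.
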(event `Init`
  (params (Player :type "SceneComponent Object Reference") (HandPos :type "Vector Structure") (FrontPos :type "Vector Structure"))
  (`NiagaraFunctionLibrary.SpawnSystemAttached` "/Game/_FunkyMagic/_water/NS_water_splash.NS_water_splash" Player "None" (- HandPos (0.0 0.0 50.0)) (struct) "KeepRelativeOffset")
  (`KismetSystemLibrary.Delay` 1.0)
  (`ProjectileMovementComponent.SetVelocityInLocalSpace` (`self.ProjectileMovement`) (`KismetMathLibrary.MakeVector` 700.0 0.0 (* (.z FrontPos) 700.0)))
  (`ActorComponent.Activate` (`self.ProjectileMovement`) false))

(event `self.Sphere.OnComponentHit`
  (params (HitComponent :type "PrimitiveComponent Object Reference") (OtherActor :type "Actor Object Reference") (OtherComp :type "PrimitiveComponent Object Reference") (NormalImpulse :type "Vector Structure") (Hit :type "HitResult Structure (by ref)"))
  (bind _returnvalue (`|SpawnActorFromClass` "/Game/_FunkyMagic/_water/BP_WaterPool.BP_WaterPool_C" (`KismetMathLibrary.MakeTransform` (+ (* (`.ImpactPoint` (`GameplayStatics.BreakHitResult` Hit)) (1.0 1.0 0.0)) (0.0 0.0 1.0))) "Undefined" "MultiplyWithRoot" null null))
  (`/Game/_FunkyMagic/_water/BP_WaterPool.Init` _returnvalue)
  (`self.K2_DestroyActor`))

(fn `UserConstructionScript`)
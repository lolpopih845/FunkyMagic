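; BP_FireBall is a fireball actor that launches a Niagara effect after a short charge delay, then cleans itself up.
; Init stores a direction vector, waits, fires, and destroys the actor after a longer delay.
; Firing sets the effect's Speed vector, fixed along X with Z scaled from the stored direction, detaches the actor in world space, and activates the effect.
; The graph contains no movement, collision or damage logic.
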(event `WaitToDestroy`
  (`self.K2_DestroyActor`))

(event `FireFireball`
  (`NiagaraComponent.SetVariableVec3` (`self.NS_Fireball1`) "Speed" (`KismetMathLibrary.MakeVector` 5000.0 0.0 (* (.z (`self.FrontPos`)) 5000.0)))
  (`self.K2_DetachFromActor` "KeepWorld" "KeepWorld" "KeepWorld")
  (`ActorComponent.Activate` (`self.NS_Fireball1`) false))

(event `Init`
  (params (FrontPos :type "Vector Structure"))
  (set `self.FrontPos` FrontPos)
  (`KismetSystemLibrary.Delay` 1.5)
  (`self.FireFireball`)
  (`KismetSystemLibrary.Delay` 7.5)
  (`self.WaitToDestroy`))

(fn `UserConstructionScript`)
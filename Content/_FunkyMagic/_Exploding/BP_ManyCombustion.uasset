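; BP_ManyCombustion is a short-lived effect actor that plays a burst of repeated combustion explosions around its location.
; On Tick it counts down a cooldown and spawns a scaled-up NS_Combustion system at a random-direction, fixed-radius offset from the actor.
; A counter tracks the spawns, and the actor destroys itself once it passes the limit.
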(event `self.ReceiveTick`
  (params (DeltaSeconds :type "Float (single-precision)"))
  (if (> (`self.num`) 15)
    (`self.K2_DestroyActor`)
    (else
      (bind _output_get (set `self.cd` (- (`self.cd`) DeltaSeconds)))
      (if (< _output_get 0.0)
        (set `self.cd` 0.15)
        (`NiagaraFunctionLibrary.SpawnSystemAtLocation` "/Game/_FunkyMagic/_Exploding/NS_Combustion.NS_Combustion" (+ (`self.K2_GetActorLocation`) (* (`KismetMathLibrary.RandomUnitVector`) 150.0)) (struct) (15.0 15.0 15.0))
        (set `self.num` (+ (`self.num`) 1))))))

(fn `UserConstructionScript`)